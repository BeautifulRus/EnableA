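; BP_Generator is a destructible generator actor whose health is reported to the in-game HUD.
; On BeginPlay it caches BP_HUDInGame, then a timeline bobs the mesh along Z, with a FlipFlop alternating reverse and forward playback after short pauses.
; AnyDamage subtracts from current HP, passes current and max HP to the HUD's in-game widget, and destroys the actor once HP runs out.
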(event Game|Damage|EventAnyDamage
  (params (Damage :type Float%20%28single-precision%29) (DamageType :type Damage%20Type%20Object%20Reference) (InstigatedBy :type Controller%20Object%20Reference) (DamageCauser :type Actor%20Object%20Reference))
  (bind _output_get (Variables|Default|SetCurentHP (- (Variables|Default|GetCurentHP) Damage)))
  (Default|GeneratorDamaged (Variables|/Game/EnableA/Game/HUDInGame/BPC_AllUMGInGame.BPC_AllUMGInGame_C|GetRefWInGame (Variables|/Game/EnableA/Game/HUDInGame/BP_HUDInGame.BP_HUDInGame_C|GetBPC_AllUMGInGame (Variables|Default|GetRef%20BP%20HUDIn%20Game))) (Variables|Default|GetGeneratorMaxHP) _output_get)
  (if (<= _output_get 0.0)
    (Actor|DestroyActor)))

(event EventBeginPlay
  (bind _asbp_hudin_game (Utilities|Casting|CastToBP_HUDInGame (HUD|GetHUD (Game|GetPlayerController 0))))
  (Variables|Default|SetRef%20BP%20HUDIn%20Game _asbp_hudin_game)
  (bind _newtrack_0 (Timeline|Timeline_0 PlayFromStart)
    (:Update
      (Transformation|SetRelativeLocation (Variables|Default|GetStaticMesh) (Math|Vector|MakeVector 0.0 0.0 _newtrack_0) false false))
    (:Finished
      (Utilities|FlowControl|FlipFlop
        (:A
          (Utilities|FlowControl|Delay 0.2)
          (Timeline|Timeline_0 Reverse))
        (:B
          (Utilities|FlowControl|Delay 0.2)
          (Timeline|Timeline_0 PlayFromStart))))))

(fn ConstructionScript)