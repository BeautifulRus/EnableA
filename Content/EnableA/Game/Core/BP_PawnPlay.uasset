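; BP_PawnPlay is the player hero pawn, with axis movement, cursor-facing rotation, shield, health and weapon pickup.
; Tick rotates the hero, regenerates shield and health per frame, and pushes both to the HUD.
; Overlaps identify weapons by tag and a counter-driven cast chain; only pistols attach to the Arrow and respond to Fire.
; A timed speed buff works, while health damage, weapon switching and most non-weapon pickups are unfinished.
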(event OnComponentBeginOverlap(re)
  (params (OverlappedComponent :type Primitive%20Component%20Object%20Reference) (OtherActor :type Actor%20Object%20Reference) (OtherComp :type Primitive%20Component%20Object%20Reference) (OtherBodyIndex :type Integer) (bFromSweep :type Boolean) (SweepResult :type Hit%20Result%20Structure%20%28by%20ref%29))
  ;[1 1 1] Определение объекта, с которым герой втупил в коллизию
  ;;[1 0.9334 0.1511] Определение оружия
  (if (Actor|ActorHasTag OtherActor "Weapon")
    (Variables|Default|SetIntForSwitchForCastWeapon 0)
    (if (Actor|ActorHasTag OtherActor "Pistol") ; Pistol
      ;;;[0 0.2446 1] Pistol
      (switch int (Variables|Default|GetIntForSwitchForCastWeapon) :!label _label
        (:0
          (bind _asbp_weapon_pistol_1 (Utilities|Casting|CastToBP_WeaponPistol1 OtherActor)
            (:then
              (Default|ActorIsAttached (stale _asbp_weapon_pistol_5) :!label _label_2)
              (Transformation|AttachComponentToComponent (stale _asbp_weapon_pistol_2) (Variables|Default|GetArrow) "" "SnapToTarget" "SnapToTarget" "SnapToTarget" true))
            (:CastFailed
              (Math|Integer|IncrementInt (Variables|Default|GetIntForSwitchForCastWeapon) :!label _label_3
                (:%20%20
                  (goto _label))))))
        (:1
          (bind _asbp_weapon_pistol_2 (Utilities|Casting|CastToBP_WeaponPistol2 OtherActor)
            (:then
              (goto _label_2))
            (:CastFailed
              (goto _label_3))))
        (:2
          (bind _asbp_weapon_pistol_3 (Utilities|Casting|CastToBP_WeaponPistol3 OtherActor)
            (:then
              (goto _label_2))
            (:CastFailed
              (goto _label_3))))
        (:3
          (bind _asbp_weapon_pistol_4 (Utilities|Casting|CastToBP_WeaponPistol4 OtherActor)
            (:then
              (goto _label_2))
            (:CastFailed
              (goto _label_3))))
        (:4
          (bind _asbp_weapon_pistol_5 (Utilities|Casting|CastToBP_WeaponPistol5 OtherActor)
            (:then
              (goto _label_2))
            (:CastFailed
              (goto _label_3))))
        (:5
          (Development|PrintString "fail switch Pistol cast to 
BP_PawnPlay" true true "(R=1.000000,G=0.021740,B=0.000000,A=1.000000)" 1e+01)))
      (elif (Actor|ActorHasTag OtherActor "Rifle") ; Rifle
        ;;;[0 0.2462 1] Rifle
        (switch int (Variables|Default|GetIntForSwitchForCastWeapon) :!label _label_4
          (:0
            (bind _asbp_weapon_rifle_1 (Utilities|Casting|CastToBP_WeaponRifle1 OtherActor)
              (:then
                (Default|ActorIsAttached _asbp_weapon_rifle_1))
              (:CastFailed
                (Math|Integer|IncrementInt (Variables|Default|GetIntForSwitchForCastWeapon) :!label _label_5
                  (:%20%20
                    (goto _label_4))))))
          (:1
            (bind _asbp_weapon_rifle_2 (Utilities|Casting|CastToBP_WeaponRifle2 OtherActor)
              (:then
                (Default|ActorIsAttached _asbp_weapon_rifle_2))
              (:CastFailed
                (goto _label_5))))
          (:2
            (bind _asbp_weapon_rifle_3 (Utilities|Casting|CastToBP_WeaponRifle3 OtherActor)
              (:then
                (Default|ActorIsAttached _asbp_weapon_rifle_3))
              (:CastFailed
                (goto _label_5))))
          (:3
            (bind _asbp_weapon_rifle_4 (Utilities|Casting|CastToBP_WeaponRifle4 OtherActor)
              (:then
                (Default|ActorIsAttached _asbp_weapon_rifle_4))
              (:CastFailed
                (goto _label_5))))
          (:4
            (bind _asbp_weapon_rifle_5 (Utilities|Casting|CastToBP_WeaponRifle5 OtherActor)
              (:then
                (Default|ActorIsAttached _asbp_weapon_rifle_5))
              (:CastFailed
                (goto _label_5))))
          (:5
            (Development|PrintString "fail switch Rifle cast to 
BP_PawnPlay" true true "(R=1.000000,G=0.021740,B=0.000000,A=1.000000)" 1e+01)))
        (elif (Actor|ActorHasTag OtherActor "Shotgun") ; Shotgun
          ;;;[0 0.2462 1] Shotgun
          (switch int (Variables|Default|GetIntForSwitchForCastWeapon) :!label _label_6
            (:0
              (bind _asbp_weapon_shotgun_1 (Utilities|Casting|CastToBP_WeaponShotgun1 OtherActor)
                (:then
                  (Default|ActorIsAttached _asbp_weapon_shotgun_1))
                (:CastFailed
                  (Math|Integer|IncrementInt (Variables|Default|GetIntForSwitchForCastWeapon) :!label _label_7
                    (:%20%20
                      (goto _label_6))))))
            (:1
              (bind _asbp_weapon_shotgun_2 (Utilities|Casting|CastToBP_WeaponShotgun2 OtherActor)
                (:then
                  (Default|ActorIsAttached _asbp_weapon_shotgun_2))
                (:CastFailed
                  (goto _label_7))))
            (:2
              (bind _asbp_weapon_shotgun_3 (Utilities|Casting|CastToBP_WeaponShotgun3 OtherActor)
                (:then
                  (Default|ActorIsAttached _asbp_weapon_shotgun_3))
                (:CastFailed
                  (goto _label_7))))
            (:3
              (Development|PrintString "fail switch Shotgun cast to 
BP_PawnPlay" true true "(R=1.000000,G=0.021740,B=0.000000,A=1.000000)" 1e+01)))
          (elif (Actor|ActorHasTag OtherActor "Sniper") ; Sniper
            ;;;[0 0.2462 1] Sniper
            (switch int (Variables|Default|GetIntForSwitchForCastWeapon) :!label _label_8
              (:0
                (bind _asbp_weapon_sniper_1 (Utilities|Casting|CastToBP_WeaponSniper1 OtherActor)
                  (:then
                    (Default|ActorIsAttached _asbp_weapon_sniper_1))
                  (:CastFailed
                    (Math|Integer|IncrementInt (Variables|Default|GetIntForSwitchForCastWeapon) :!label _label_9
                      (:%20%20
                        (goto _label_8))))))
              (:1
                (bind _asbp_weapon_sniper_2 (Utilities|Casting|CastToBP_WeaponSniper2 OtherActor)
                  (:then
                    (Default|ActorIsAttached _asbp_weapon_sniper_2))
                  (:CastFailed
                    (goto _label_9))))
              (:2
                (bind _asbp_weapon_sniper_3 (Utilities|Casting|CastToBP_WeaponSniper3 OtherActor)
                  (:then
                    (Default|ActorIsAttached _asbp_weapon_sniper_3))
                  (:CastFailed
                    (goto _label_9))))
              (:3
                (Development|PrintString "fail switch Sniper cast to 
BP_PawnPlay" true true "(R=1.000000,G=0.021740,B=0.000000,A=1.000000)" 1e+01)))
            (else
              (Development|PrintString "this not a weapon 
BP_PawnPlay 
OnComponentBeginOverlap"))))))
    (elif (Actor|ActorHasTag OtherActor "Item")
      (bind _asbp_item_barricade (Utilities|Casting|CastToBP_ItemBarricade OtherActor))
      (else
        (if (Actor|ActorHasTag OtherActor "Chest")
          _
          (elif (Actor|ActorHasTag OtherActor "Buff")
            _
            (else
              _)))
        (Development|PrintString "не готово")))))

(event Custom|PickUpSpeedBuff
  (params (SpeedBuff :type Float%20%28single-precision%29) (LifetimeBuff :type Float%20%28single-precision%29))
  ;[1 1 1] Пример того, как работает бафф
  (bind _output_get (Variables|BufsInformation|SetSpeedBuff SpeedBuff))
  (Variables|/Script/Engine.FloatingPawnMovement|SetMaxSpeed (Variables|Default|GetFloatingPawnMovement) (* (Variables|HeroInformation|GetHeroMovementSpeed) _output_get))
  (Utilities|FlowControl|Delay LifetimeBuff)
  (Variables|/Script/Engine.FloatingPawnMovement|SetMaxSpeed (Variables|Default|GetFloatingPawnMovement) (Variables|HeroInformation|GetHeroMovementSpeed)))

(event Custom|HeroDamaged/HealthLogic
  (params (InputDamage :type Float%20%28single-precision%29))
  ;[1 1 1] Это всё место под реализацю логики героя и его характеристик
)

(event Custom|ShiledRegenerationDelay
  ;[1 1 1] Это всё место под реализацю логики героя и его характеристик
  ;;[1 1 1] Shield
  (Utilities|FlowControl|Delay (Variables|HeroInformation|GetWaitingBeforeRegeneratingTheShield))
  (Variables|HeroInformation|SetHasHeroDamadged false))

(event Custom|HeroPickUpWeapon
  ;[1 1 1] Это всё место под реализацю логики героя и его характеристик
  ;;[1 1 1] Weapon
  (if (not (>= (Variables|Default|GetAmountWeaponOnHero) 3))
    (Math|Integer|IncrementInt (Variables|Default|GetAmountWeaponOnHero)
      (:%20%20
        (Transformation|AttachComponentToComponent 0 "None" "KeepRelative" "KeepRelative" "KeepRelative" true)))))

(event Custom|SwitchWeapon
  ;[1 1 1] Это всё место под реализацю логики героя и его характеристик
  ;;[1 1 1] Weapon
)

(event Custom|HeroDamadged/ShieldLogic
  (params (InputDamage :type Float%20%28single-precision%29))
  ;[1 1 1] Это всё место под реализацю логики героя и его характеристик
  ;;[1 1 1] Shield
  (Variables|HeroInformation|SetHasHeroDamadged true)
  (if (< (- (- InputDamage (Variables|HeroInformation|GetArmor)) (Variables|HeroInformation|GetShieldInTime)) 0.0)
    (Variables|HeroInformation|SetShieldInTime 0.0)
    (else
      (Variables|HeroInformation|SetShieldInTime (- (- InputDamage (Variables|HeroInformation|GetArmor)) (Variables|HeroInformation|GetShieldInTime))))))

(event EventBeginPlay
  ;[1 1 1] Придание базовых настроек персонажу и получение на будущее необходимых на объекты ссылок
  (Variables|/Script/Engine.FloatingPawnMovement|SetMaxSpeed (Variables|Default|GetFloatingPawnMovement) (Variables|HeroInformation|GetHeroMovementSpeed))
  (Variables|HeroInformation|SetShieldInTime (Variables|HeroInformation|GetMaxShield))
  (Variables|HeroInformation|SetHealthInTime (Variables|HeroInformation|GetMaxHealth))
  (bind _asbp_hudin_game (Utilities|Casting|CastToBP_HUDInGame (HUD|GetHUD (Game|GetPlayerController 0))))
  (Variables|Default|SetRefBP_HUDInGame _asbp_hudin_game))

(event EventTick
  (params (DeltaSeconds :type Float%20%28single-precision%29))
  ;[1 1 1] BasedLogic
  (CallFunction|HeroRotatetoCursor DeltaSeconds)
  (CallFunction|ShieldRegeneration)
  (CallFunction|HealthRegeneration)
  (Default|UpdateHealth&SheldBar (Variables|/Game/EnableA/Game/HUDInGame/W_InGame.W_InGame_C|GetW_HeathPointAndShield (Variables|/Game/EnableA/Game/HUDInGame/BPC_AllUMGInGame.BPC_AllUMGInGame_C|GetRefWInGame (Variables|/Game/EnableA/Game/HUDInGame/BP_HUDInGame.BP_HUDInGame_C|GetBPC_AllUMGInGame (Variables|Default|GetRefBP_HUDInGame)))) (Variables|HeroInformation|GetShieldInTime) (Variables|HeroInformation|GetHealthInTime)))

(event Input|ActionEvents|InputActionFire
  (params (Key :type Key%20Structure :default "None"))
  ;[1 1 1] Определение объекта, с которым герой втупил в коллизию
  ;;[1 1 1] В будущем, сделать переключение оружия на руки и за спину, и в зависимости от этого стрелять только из одного оружия в руках
  (:Pressed
    (if true
      (Default|Fire (stale OnComponentBeginOverlap(re) _asbp_weapon_pistol_2) (Variables|HeroInformation|GetDamage))))
  (:Released
    (Default|StopFire(ForAutoWeapon) (stale OnComponentBeginOverlap(re) _asbp_weapon_pistol_2))))

(event Input|AxisEvents|InputAxisMoveUpward
  (params (AxisValue :type Float%20%28single-precision%29))
  ;[1 1 1] HeroMovement
  (Class|PawnMovementComponent|AddInputVector (Variables|Default|GetFloatingPawnMovement) (Math|Vector|MakeVector AxisValue (stale Input|AxisEvents|InputAxisMoveLeft AxisValue) 0.0) false))

(event Input|AxisEvents|InputAxisMoveLeft
  (params (AxisValue :type Float%20%28single-precision%29))
  ;[1 1 1] HeroMovement
  (Class|PawnMovementComponent|AddInputVector (Variables|Default|GetFloatingPawnMovement) (Math|Vector|MakeVector (stale Input|AxisEvents|InputAxisMoveUpward AxisValue) AxisValue 0.0) false))

(event Input|MouseEvents|RightMouseButton
  (params (Key :type Key%20Structure :default "None"))
  (:Pressed
    (Default|Qwer (stale OnComponentBeginOverlap(re) _asbp_item_barricade))))

(fn ConstructionScript)

(fn HeroRotatetoCursor
  (params (XWire :type Float%20%28single-precision%29))
  (Variables|/Script/Engine.PlayerController|SetbShowMouseCursor (Game|GetPlayerController 0) true)
  (Transformation|SetActorRotation self (Math|Rotator|MakeRotator 0.0 0.0 (.yaw (Math|Rotator|FindLookatRotation (Transformation|GetActorLocation) (.location (.HitResult (Game|Player|GetHitResultUnderCursorbyChannel (Game|GetPlayerController 0) "TraceTypeQuery1" true))))))))

(fn ShieldRegeneration
  (if (not (Variables|HeroInformation|GetHasHeroDamadged))
    ;[1 1 1] Проверка на баг
    (if (> (Variables|HeroInformation|GetShieldInTime) (Variables|HeroInformation|GetMaxShield))
      (if (not (Variables|HeroInformation|GetHasShieldBuff))
        (Variables|HeroInformation|SetShieldInTime 0.0)
        (CallFunction|ShiledRegenerationDelay))
      (elif (> (+ (/ (Variables|HeroInformation|GetShieldRegeneration) 6e+01) (Variables|HeroInformation|GetShieldInTime)) (Variables|HeroInformation|GetMaxShield))
        (Variables|HeroInformation|SetShieldInTime (Variables|HeroInformation|GetMaxShield))
        (else
          (Variables|HeroInformation|SetShieldInTime (+ (/ (Variables|HeroInformation|GetShieldRegeneration) 6e+01) (Variables|HeroInformation|GetShieldInTime))))))))

(fn HealthRegeneration
  (if (> (+ (/ (Variables|HeroInformation|GetHealthRegeneration) 6e+01) (Variables|HeroInformation|GetHealthInTime)) (Variables|HeroInformation|GetMaxHealth))
    (Variables|HeroInformation|SetHealthInTime (Variables|HeroInformation|GetMaxHealth))
    (else
      (Variables|HeroInformation|SetHealthInTime (+ (/ (Variables|HeroInformation|GetHealthRegeneration) 6e+01) (Variables|HeroInformation|GetHealthInTime))))))