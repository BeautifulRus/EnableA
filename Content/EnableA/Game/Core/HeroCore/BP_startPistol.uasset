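; Starting pistol Blueprint that handles firing, fire-rate gating and magazine reloading.
; FireStartPistol runs a debug-drawn Visibility line trace forward from the Arrow component with a fixed end height; the hit result is unused.
; A ready flag blocks firing during the one-second cooldown, after which ammo decrements.
; Firing on an empty magazine instead waits out the reload delay and refills to capacity.
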(event Custom|FireStartPistol
  (bind _arrow (Variables|Default|GetArrow))
  (bind _arrow_2 (Variables|Default|GetArrow))
  (bind _returnvalue (Math|Vector|GetForwardVector _arrow))
  (bind _returnvalue_2 (Transformation|GetWorldLocation _arrow_2))
  (bind _returnvalue_3 (* _returnvalue 1.3e+03))
  (bind _returnvalue_4 (+ _returnvalue_3 _returnvalue_2))
  (if (Variables|Default|GetReadyToShoot)
    (Variables|Default|SetReadyToShoot false)
    (if (<= (Variables|Default|GetNumberOf%20Remaining%20AmmoInTheMagazine) 0)
      (Utilities|FlowControl|Delay (Variables|Default|GetRemovalAndReloading))
      (Variables|Default|SetNumberOf%20Remaining%20AmmoInTheMagazine (Variables|Default|GetMagazineCapacity))
      (Variables|Default|SetReadyToShoot true)
      (else
        (Collision|LineTraceByChannel _returnvalue_2 (Math|Vector|MakeVector (.x _returnvalue_4) (.y _returnvalue_4) 1.1e+02) "TraceTypeQuery1" false 0 "ForDuration")
        (Utilities|FlowControl|Delay 1.0)
        (Variables|Default|SetReadyToShoot true)
        (Math|Integer|DecrementInt (Variables|Default|GetNumberOf%20Remaining%20AmmoInTheMagazine))))))

(event EventBeginPlay
  (Variables|Default|SetNumberOf%20Remaining%20AmmoInTheMagazine (Variables|Default|GetMagazineCapacity)))

(event Collision|EventActorBeginOverlap
  (params (OtherActor :type Actor%20Object%20Reference)))

(event EventTick
  (params (DeltaSeconds :type Float%20%28single-precision%29)))

(fn ConstructionScript)