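; Starting pistol weapon Blueprint that fires projectiles from a limited magazine.
; FireStartPistol spawns a BP_PistolProjectileMovement at the Arrow's transform, gated by a ReadyToShoot flag that resets after a zero-length delay.
; Firing on an empty magazine instead waits out the reload delay and refills to MagazineCapacity, which also sets the starting ammo.
; After each shot, a one-second delay precedes destroying the spawned projectile if still valid.
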(event Custom|FireStartPistol
  (if (Variables|Default|GetReadyToShoot)
    (Variables|Default|SetReadyToShoot false)
    (if (<= (Variables|Default|GetNumberOf%20Remaining%20AmmoInTheMagazine) 0)
      (Utilities|FlowControl|Delay (Variables|Default|GetRemovalAndReloading))
      (Variables|Default|SetNumberOf%20Remaining%20AmmoInTheMagazine (Variables|Default|GetMagazineCapacity))
      (Variables|Default|SetReadyToShoot true)
      (else
        (bind _returnvalue (Game|SpawnActorfromClass "/Game/EnableA/Game/Core/HeroCore/HeroWeapon/BP_PistolProjectileMovement.BP_PistolProjectileMovement_C" (Transformation|GetWorldTransform (Variables|Default|GetArrow)) "Undefined" 0 0))
        (Utilities|FlowControl|Delay 0.0)
        (Variables|Default|SetReadyToShoot true)
        (Math|Integer|DecrementInt (Variables|Default|GetNumberOf%20Remaining%20AmmoInTheMagazine)
          (:%20%20
            (Utilities|FlowControl|Delay 1.0)
            (Utilities|IsValid _returnvalue
              (:Is%20Valid
                (Actor|DestroyActor _returnvalue)))))))))

(event EventBeginPlay
  (Variables|Default|SetNumberOf%20Remaining%20AmmoInTheMagazine (Variables|Default|GetMagazineCapacity)))

(event Collision|EventActorBeginOverlap
  (params (OtherActor :type Actor%20Object%20Reference)))

(event EventTick
  (params (DeltaSeconds :type Float%20%28single-precision%29)))

(fn ConstructionScript)