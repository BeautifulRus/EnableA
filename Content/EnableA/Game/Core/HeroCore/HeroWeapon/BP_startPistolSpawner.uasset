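; Component that gives its owning BP_PawnPlay a starting pistol and lets it be removed or respawned.
; On BeginPlay it casts the owner to BP_PawnPlay, spawns BP_startPistol at the mesh's "ForGun" socket and attaches it there.
; StartPistolOff destroys the pistol and clears its reference, while StartPistolOnn runs the same spawn-and-attach logic to create a new one.
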(event Custom|StartPistolOff
  (Actor|DestroyActor (stale Custom|StartPistolOnn _returnvalue))
  (Variables|Default|SetStartPistol 0))

(event Custom|StartPistolOnn
  (bind _returnvalue (Game|SpawnActorfromClass "/Game/EnableA/Game/Core/HeroCore/HeroWeapon/BP_startPistol.BP_startPistol_C" (Transformation|GetSocketTransform (Variables|/Script/Engine.Character|GetMesh (stale EventBeginPlay _asbp_pawn_play)) "ForGun" "RTS_World") "Undefined" 0 0))
  (bind _output_get (Variables|Default|SetStartPistol _returnvalue))
  (Transformation|AttachComponentToComponent _output_get (Variables|/Script/Engine.Character|GetMesh (stale EventBeginPlay _asbp_pawn_play)) "ForGun" "KeepWorld" "KeepWorld" "KeepWorld" true))

(event EventBeginPlay
  (bind _asbp_pawn_play (Utilities|Casting|CastToBP_PawnPlay (Components|GetOwner)))
  (bind _returnvalue (Game|SpawnActorfromClass "/Game/EnableA/Game/Core/HeroCore/HeroWeapon/BP_startPistol.BP_startPistol_C" (Transformation|GetSocketTransform (Variables|/Script/Engine.Character|GetMesh _asbp_pawn_play) "ForGun" "RTS_World") "Undefined" 0 0))
  (bind _output_get (Variables|Default|SetStartPistol _returnvalue))
  (Transformation|AttachComponentToComponent _output_get (Variables|/Script/Engine.Character|GetMesh _asbp_pawn_play) "ForGun" "KeepWorld" "KeepWorld" "KeepWorld" true))

(event EventTick
  (params (DeltaSeconds :type Float%20%28single-precision%29)))