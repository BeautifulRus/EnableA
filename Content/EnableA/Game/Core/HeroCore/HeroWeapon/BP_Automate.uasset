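; BP_Automate is the hero's automatic weapon, spawning BP_PistolProjectileMovement projectiles from its Arrow while firing.
; FireAutomate loops through a short Delay until StopFireAutomate clears ReadyToShoot, decrementing magazine ammo per shot.
; An empty magazine refills after the RemovalAndReloading delay, without re-entering the fire loop.
; A parallel one-second Delay destroys the spawned projectile reference, sharing one latent node across rapid shots.
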(event Custom|FireAutomate
  (Variables|Default|SetReadyToShoot true)
  (if (Variables|Default|GetReadyToShoot) :!label _label
    (Variables|Default|SetReadyToShoot false)
    (if (<= (Variables|Default|GetNumberOf%20Remaining%20AmmoInTheMagazine) 0)
      (Utilities|FlowControl|Delay (Variables|Default|GetRemovalAndReloading))
      (Variables|Default|SetNumberOf%20Remaining%20AmmoInTheMagazine (Variables|Default|GetMagazineCapacity))
      (Variables|Default|SetReadyToShoot true)
      (else
        (bind _returnvalue (Game|SpawnActorfromClass "/Game/EnableA/Game/Core/HeroCore/HeroWeapon/BP_PistolProjectileMovement.BP_PistolProjectileMovement_C" (Transformation|GetWorldTransform (Variables|Default|GetArrow)) "Undefined" 0 0))
        (Variables|Default|SetReadyToShoot true)
        (Math|Integer|DecrementInt (Variables|Default|GetNumberOf%20Remaining%20AmmoInTheMagazine)
          (:%20%20
            (Utilities|FlowControl|Sequence
              (:then_0
                (Utilities|FlowControl|Delay 0.05)
                (goto _label))
              (:then_1
                (Utilities|FlowControl|Delay 1.0)
                (Utilities|IsValid _returnvalue
                  (:Is%20Valid
                    (Actor|DestroyActor _returnvalue)))))))))))

(event Custom|StopFireAutomate
  (Variables|Default|SetReadyToShoot false))

(event EventBeginPlay
  (Variables|Default|SetNumberOf%20Remaining%20AmmoInTheMagazine (Variables|Default|GetMagazineCapacity)))

(event Collision|EventActorBeginOverlap
  (params (OtherActor :type Actor%20Object%20Reference)))

(fn ConstructionScript)