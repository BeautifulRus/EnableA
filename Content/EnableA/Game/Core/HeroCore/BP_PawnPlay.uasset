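; Player hero pawn for a top-down shooter, handling cursor-facing movement, a timed speed-boost dash, shooting and health.
; Tick rotates the hero, regenerates health at an assumed 60 fps and updates the HUD bar.
; Capsule overlaps use actor tags to attach or upgrade SteamPack and HealingCrystal items, while HeroFindAutomate replaces the pistol with an automatic.
; Armor reduces damage, YOUWILLDIE repeats damage until death, and shield regeneration is defined but never called.
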(event OnComponentBeginOverlap(CapsuleComponent)
  (params (OverlappedComponent :type Primitive%20Component%20Object%20Reference) (OtherActor :type Actor%20Object%20Reference) (OtherComp :type Primitive%20Component%20Object%20Reference) (OtherBodyIndex :type Integer) (bFromSweep :type Boolean) (SweepResult :type Hit%20Result%20Structure%20%28by%20ref%29))
  ;[0.2573 1 0.1338] Определение объекта, с которым герой втупил в коллизию
  (Variables|important,butIdon'tknowwheretoputit|SetIntForSwitchForCastWeapon 0 :!pinned true) ; не удаляй
  (if (Actor|ActorHasTag OtherActor "Weapon")
    (Utilities|IsValid 0
      (:Is%20Not%20Valid
        (if (Actor|ActorHasTag OtherActor "Pistol") ; Pistol
          _)))
    (elif (Actor|ActorHasTag OtherActor "Item")
      (if (Actor|ActorHasTag OtherActor "Active")
        (bind _asbp_item_steam_pack (Utilities|Casting|CastToBP_ItemSteamPack OtherActor))
        (if (Variables|ActiveItemsAdded|GetSteamPuckAdded)
          (Actor|DestroyActor _asbp_item_steam_pack)
          (Default|UpgradeItem (Variables|RefActiveItems|GetRefSteamPuck))
          (else
            (Default|AttachItem&DisableCollision _asbp_item_steam_pack)
            (Variables|ActiveItemsAdded|SetSteamPuckAdded true)
            (Variables|RefActiveItems|SetRefSteamPuck _asbp_item_steam_pack)
            (Utilities|FlowControl|Sequence
              (:then_0
                (Utilities|FlowControl|Gate true) ; enters at Open
              )
              (:then_1
                (Utilities|FlowControl|DoOnce false
                  (:Completed
                    (Default|AddNewActiveItem (Variables|/Game/EnableA/Game/HUDInGame/W_InGame.W_InGame_C|GetW_ItemsActive (Variables|/Game/EnableA/Game/HUDInGame/BPC_AllUMGInGame.BPC_AllUMGInGame_C|GetRefWInGame (Variables|/Game/EnableA/Game/HUDInGame/BP_HUDInGame.BP_HUDInGame_C|GetBPC_AllUMGInGame (Variables|Important,ButIDon'tKnowWhereToPutIt|GetRefBP_HUDInGame)))) "SteamPack")))))))
        (elif (Actor|ActorHasTag OtherActor "Passive")
          (bind _asbp_item_healing_crystal (Utilities|Casting|CastToBP_ItemHealingCrystal OtherActor))
          (if (Variables|PassiveItemsAdded|GetHealingCrystalAdded)
            (Default|UpgradeItem (Variables|RefPassiveItems|GetRefHealingCrystal))
            (Actor|DestroyActor _asbp_item_healing_crystal)
            (else
              (Default|AttachItem&DisableCollision _asbp_item_healing_crystal)
              (Default|AddItem (Variables|/Game/EnableA/Game/HUDInGame/BPC_AllUMGInGame.BPC_AllUMGInGame_C|GetRefWInGame (Variables|/Game/EnableA/Game/HUDInGame/BP_HUDInGame.BP_HUDInGame_C|GetBPC_AllUMGInGame (Variables|Important,ButIDon'tKnowWhereToPutIt|GetRefBP_HUDInGame))) "HealingCrystal")
              (Variables|RefPassiveItems|SetRefHealingCrystal _asbp_item_healing_crystal)
              (Variables|PassiveItemsAdded|SetHealingCrystalAdded true))))))))

(event Custom|SteamPuckUse
  ;[1 1 1] Это всё место под реализацю логики героя и его характеристик
  (Variables|/Script/Engine.CharacterMovementComponent|SetMaxWalkSpeed (Variables|Character|GetCharacterMovement) (Variables|HeroInformation|GetHeroMovementSpeed)))

(event Custom|HeroFindAutomate
  ;[1 1 1] Это всё место под реализацю логики героя и его характеристик
  ;;[1 1 1] В будущем, сделать переключение оружия на руки и за спину, и в зависимости от этого стрелять только из одного оружия в руках
  (if (Variables|Default|GetIsPistol)
    (Variables|Default|SetIsPistol false)
    (Default|StartPistolOff (Variables|Default|GetBP_startPistolSpawner))
    (Utilities|FlowControl|Delay 0.2)
    (bind _returnvalue (Game|SpawnActorfromClass "/Game/EnableA/Game/Core/HeroCore/HeroWeapon/BP_Automate.BP_Automate_C" (Transformation|GetActorTransform) "Undefined" 0 0))
    (Transformation|AttachComponentToComponent _returnvalue (Variables|Default|GetArrow) "None" "SnapToTarget" "SnapToTarget" "SnapToTarget" true)))

(event Custom|YOU%20WILL%20DIE
  (params (Damage :type Float%20%28single-precision%29))
  (bind _armor (Variables|HeroInformation|GetArmor))
  (bind _returnvalue (- Damage _armor))
  ;[1 1 1] Это всё место под реализацю логики героя и его характеристик
  (Development|PrintString "mission failure 
you will die" true true "(R=0.843359,G=0.000000,B=1.000000,A=1.000000)" 2e+01)
  (if (not (<= _returnvalue 0.0)) :!label _label
    (Audio|PlaySound2D "/Game/EnableA/Game/Into_the_Void/Insects/Insects_Atack/Claws_in_Flesh.Claws_in_Flesh" 0.2 1.0 0.0 0 0)
    (bind _output_get (Variables|HeroInformation|SetHealthCurent (- (Variables|HeroInformation|GetHealthCurent) _returnvalue)))
    (if (<= _output_get 0.0)
      (Development|PrintString "YOU ARE DEAD" true true "(R=1.000000,G=0.000000,B=0.000000,A=1.000000)" 2e+02)
      (Input|SetInputModeUIOnly (Game|GetPlayerController 0) 0 "DoNotLock")
      (Input|DisableInput (Game|GetPlayerController 0))
      (else
        (Utilities|FlowControl|Delay 0.7)
        (goto _label)))))

(event Custom|HeroPickUpWeapon
  ;[1 1 1] Weapon
  (if (not (>= (Variables|Weapon|GetAmountWeaponOnHero) 3))
    (Math|Integer|IncrementInt (Variables|Weapon|GetAmountWeaponOnHero)
      (:%20%20
        (Transformation|AttachComponentToComponent 0 "None" "KeepRelative" "KeepRelative" "KeepRelative" true)))))

(event Custom|SwitchWeapon
  ;[1 1 1] Weapon
)

(event EventBeginPlay
  (bind _heromovementspeed (Variables|HeroInformation|GetHeroMovementSpeed))
  ;[1 1 1] Придание базовых настроек персонажу и получение на будущее необходимых на объекты ссылок
  (Variables|/Script/Engine.CharacterMovementComponent|SetMaxWalkSpeed (Variables|Character|GetCharacterMovement) _heromovementspeed)
  (Variables|HeroInformation|SetHealthCurent (Variables|HeroInformation|GetMaxHealth))
  (Variables|HeroInformation|SetDashMovementSpeed (* _heromovementspeed 3e+01))
  (bind _asbp_hudin_game (Utilities|Casting|CastToBP_HUDInGame (HUD|GetHUD (Game|GetPlayerController 0))))
  (Variables|Important,ButIDon'tKnowWhereToPutIt|SetRefBP_HUDInGame _asbp_hudin_game)
  (bind _outactors (Actor|GetAllActorsOfClass "/Game/EnableA/Game/Core/Drill/BP_Drill.BP_Drill_C"))
  (Variables|Default|SetRefDrill (Utilities|Array|Get(acopy) _outactors))
  (bind _outactors_2 (Actor|GetAllActorsOfClass "/Game/EnableA/Game/Core/generator/BP_Generator.BP_Generator_C"))
  (Variables|Default|SetRefGenerator (Utilities|Array|Get(acopy) _outactors_2)))

(event Game|Damage|EventAnyDamage
  (params (Damage :type Float%20%28single-precision%29) (DamageType :type Damage%20Type%20Object%20Reference) (InstigatedBy :type Controller%20Object%20Reference) (DamageCauser :type Actor%20Object%20Reference))
  (bind _armor (Variables|HeroInformation|GetArmor))
  (bind _returnvalue (- Damage _armor))
  ;[1 1 1] Это всё место под реализацю логики героя и его характеристик
  ;;[1 1 1] Shield
  (if (not (<= _returnvalue 0.0))
    (Audio|PlaySound2D "/Game/EnableA/Game/Into_the_Void/Insects/Insects_Atack/Claws_in_Flesh.Claws_in_Flesh" 0.2 1.0 0.0 0 0)
    (bind _output_get (Variables|HeroInformation|SetHealthCurent (- (Variables|HeroInformation|GetHealthCurent) _returnvalue)))
    (if (<= _output_get 0.0)
      (Development|PrintString "YOU ARE DEAD" true true "(R=1.000000,G=0.000000,B=0.000000,A=1.000000)" 2e+02)
      (Input|SetInputModeUIOnly (Game|GetPlayerController 0) 0 "DoNotLock")
      (Input|DisableInput (Game|GetPlayerController 0))
      (Utilities|FlowControl|DoOnce false
        (:Completed
          (Variables|Default|Setswitch true)
          (Components|Animation|PlayAnimation (Variables|Character|GetMesh) "/Game/EnableA/Game/Core/HeroCore/HeroAnimations/MoreAnimations/Death_From_Back_Headshot_Anim.Death_From_Back_Headshot_Anim" false)
          (Audio|PlaySound2D "/Game/EnableA/Game/Into_the_Void/Soldier/Death.Death" 1.0 1.0 0.0 0 0))))))

(event EventTick
  (params (DeltaSeconds :type Float%20%28single-precision%29))
  ;[1 1 1] Это всё место под реализацю логики героя и его характеристик
  ;;[1 1 1] BasedLogic
  (if (not (Variables|Default|Getswitch))
    (CallFunction|HeroRotatetoCursor DeltaSeconds)
    (CallFunction|HealthRegeneration)
    (Default|UpdateHealth&SheldBar (Variables|/Game/EnableA/Game/HUDInGame/W_InGame.W_InGame_C|GetW_HeathPointAndShield (Variables|/Game/EnableA/Game/HUDInGame/BPC_AllUMGInGame.BPC_AllUMGInGame_C|GetRefWInGame (Variables|/Game/EnableA/Game/HUDInGame/BP_HUDInGame.BP_HUDInGame_C|GetBPC_AllUMGInGame (Variables|Important,ButIDon'tKnowWhereToPutIt|GetRefBP_HUDInGame)))) (Variables|HeroInformation|GetHealthCurent))))

(event Input|ActionEvents|InputActionDash
  (params (Key :type Key%20Structure :default "None"))
  ;[1 1 1] Это всё место под реализацю логики героя и его характеристик
  ;;[1 1 1] Dash
  (:Pressed
    (if (Variables|HeroInformation|GetDashIsReady)
      ;;;[1 1 1] Dash
      (Variables|/Script/Engine.CharacterMovementComponent|SetMaxWalkSpeed (Variables|Character|GetCharacterMovement) (Variables|HeroInformation|GetDashMovementSpeed))
      (Utilities|FlowControl|Delay (Variables|HeroInformation|GetDashDuration))
      (Variables|/Script/Engine.CharacterMovementComponent|SetMaxWalkSpeed (Variables|Character|GetCharacterMovement) (Variables|HeroInformation|GetHeroMovementSpeed))
      ;;;[1 1 1] DashRecover
      (Variables|HeroInformation|SetDashIsReady false)
      (Utilities|FlowControl|Delay (Variables|HeroInformation|GetDashCooldown))
      (Variables|HeroInformation|SetDashIsReady true))))

(event Input|ActionEvents|InputActionFire
  (params (Key :type Key%20Structure :default "None"))
  (bind _ispistol (Variables|Default|GetIsPistol))
  ;[1 1 1] Это всё место под реализацю логики героя и его характеристик
  ;;[1 1 1] В будущем, сделать переключение оружия на руки и за спину, и в зависимости от этого стрелять только из одного оружия в руках
  (:Pressed
    (if _ispistol
      (Default|FireStartPistol (Variables|/Game/EnableA/Game/Core/HeroCore/HeroWeapon/BP_startPistolSpawner.BP_startPistolSpawner_C|GetStartPistol (Variables|Default|GetBP_startPistolSpawner)))
      (else
        (Default|FireAutomate (stale Custom|HeroFindAutomate _returnvalue)))))
  (:Released
    (if (not _ispistol)
      (Default|StopFireAutomate (stale Custom|HeroFindAutomate _returnvalue)))))

(event Input|AxisEvents|InputAxisMoveUpward
  (params (AxisValue :type Float%20%28single-precision%29))
  ;[1 1 1] Это всё место под реализацю логики героя и его характеристик
  ;;[1 1 1] HeroMovement
  (Pawn|Input|AddMovementInput (Math|Vector|MakeVector AxisValue (stale Input|AxisEvents|InputAxisMoveLeft AxisValue) 0.0) 1.0 false))

(event Input|AxisEvents|InputAxisUseItem
  (params (AxisValue :type Float%20%28single-precision%29))
  ;[0.2573 1 0.1338] Определение объекта, с которым герой втупил в коллизию
  (if (== AxisValue 1.0)
    (Utilities|FlowControl|Gate true
      (:Exit
        (Default|ItemUse (Variables|RefActiveItems|GetRefSteamPuck))))))

(event Input|AxisEvents|InputAxisMoveLeft
  (params (AxisValue :type Float%20%28single-precision%29))
  ;[1 1 1] Это всё место под реализацю логики героя и его характеристик
  ;;[1 1 1] HeroMovement
)

(fn ConstructionScript)

(fn HeroRotatetoCursor
  (params (XWire :type Float%20%28single-precision%29))
  (bind _returnvalue (Transformation|GetActorLocation))
  (bind _returnvalue_2 (Game|GetPlayerController 0))
  (bind _hitresult (Game|Player|GetHitResultUnderCursorbyChannel _returnvalue_2 "TraceTypeQuery3" true))
  (bind _returnvalue_3 (Math|Rotator|FindLookatRotation _returnvalue (.location _hitresult)))
  (Variables|/Script/Engine.PlayerController|SetbShowMouseCursor (Game|GetPlayerController 0) true)
  (Transformation|SetActorRotation self (Math|Rotator|MakeRotator 0.0 0.0 (.yaw _returnvalue_3)))
  (Variables|Default|Setpisosforvard (Math|Rotator|MakeRotator (.roll _returnvalue_3) (.pitch _returnvalue_3) (.yaw _returnvalue_3)))
  (return (.location _hitresult)))

(fn ShieldRegeneration
  (if (not (Variables|HeroInformation|GetHasHeroDamadged))
    ;[1 1 1] Проверка на баг
    (if (> (Variables|HeroInformation|GetShieldCurent) (Variables|HeroInformation|GetMaxShield))
      (if (not (Variables|HeroInformation|GetHasShieldBuff))
        (Variables|HeroInformation|SetShieldCurent 0.0))
      (elif (> (+ (/ (Variables|HeroInformation|GetShieldRegeneration) 6e+01) (Variables|HeroInformation|GetShieldCurent)) (Variables|HeroInformation|GetMaxShield))
        (Variables|HeroInformation|SetShieldCurent (Variables|HeroInformation|GetMaxShield))
        (else
          (Variables|HeroInformation|SetShieldCurent (+ (/ (Variables|HeroInformation|GetShieldRegeneration) 6e+01) (Variables|HeroInformation|GetShieldCurent))))))))

(fn HealthRegeneration
  (if (> (+ (/ (Variables|HeroInformation|GetHealthRegeneration) 6e+01) (Variables|HeroInformation|GetHealthCurent)) (Variables|HeroInformation|GetMaxHealth))
    (Variables|HeroInformation|SetHealthCurent (Variables|HeroInformation|GetMaxHealth))
    (else
      (Variables|HeroInformation|SetHealthCurent (+ (/ (Variables|HeroInformation|GetHealthRegeneration) 6e+01) (Variables|HeroInformation|GetHealthCurent))))))