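; BP_startPistolSpawner spawns and removes the start pistol for the player pawn, BP_PawnPlay, that owns it.
; On BeginPlay it casts its owner to that pawn, then spawns BP_startPistol at the pawn's Arrow and attaches it there, keeping world transform.
; StartPistolOnn runs the same spawn and attach path on demand, while StartPistolOff destroys the pistol and clears the stored reference.
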(event Custom|StartPistolOff
  (Actor|DestroyActor (stale Custom|StartPistolOnn _returnvalue))
  (Variables|Default|SetStartPistol 0))

(event Custom|StartPistolOnn
  (bind _returnvalue (Game|SpawnActorfromClass "/Game/EnableA/Game/Core/HeroCore/BP_startPistol.BP_startPistol_C" (Transformation|GetWorldTransform (Variables|/Game/EnableA/Game/Core/HeroCore/BP_PawnPlay.BP_PawnPlay_C|GetArrow (stale EventBeginPlay _asbp_pawn_play))) "Undefined" 0 0))
  (bind _output_get (Variables|Default|SetStartPistol _returnvalue))
  (Transformation|AttachComponentToComponent _output_get (Variables|/Game/EnableA/Game/Core/HeroCore/BP_PawnPlay.BP_PawnPlay_C|GetArrow (stale EventBeginPlay _asbp_pawn_play)) "None" "KeepWorld" "KeepWorld" "KeepWorld" true))

(event EventBeginPlay
  (bind _asbp_pawn_play (Utilities|Casting|CastToBP_PawnPlay (Components|GetOwner)))
  (bind _returnvalue (Game|SpawnActorfromClass "/Game/EnableA/Game/Core/HeroCore/BP_startPistol.BP_startPistol_C" (Transformation|GetWorldTransform (Variables|/Game/EnableA/Game/Core/HeroCore/BP_PawnPlay.BP_PawnPlay_C|GetArrow _asbp_pawn_play)) "Undefined" 0 0))
  (bind _output_get (Variables|Default|SetStartPistol _returnvalue))
  (Transformation|AttachComponentToComponent _output_get (Variables|/Game/EnableA/Game/Core/HeroCore/BP_PawnPlay.BP_PawnPlay_C|GetArrow _asbp_pawn_play) "None" "KeepWorld" "KeepWorld" "KeepWorld" true))

(event EventTick
  (params (DeltaSeconds :type Float%20%28single-precision%29)))