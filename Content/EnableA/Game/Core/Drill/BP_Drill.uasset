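; BP_Drill is a damageable drill actor whose destruction fails the mission.
; It caches the in-game HUD on BeginPlay, then on any damage lowers its HP and sends current and max HP to the in-game widget.
; At zero HP it prints a failure message, then once damages the player pawn, calls its YOUWILLDIE function and destroys itself.
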(event EventBeginPlay
  (bind _asbp_hudin_game (Utilities|Casting|CastToBP_HUDInGame (HUD|GetHUD (Game|GetPlayerController 0))))
  (Variables|Default|SetRef%20BP%20HUDIn%20Game _asbp_hudin_game))

(event EventTick
  (params (DeltaSeconds :type Float%20%28single-precision%29)))

(event Game|Damage|EventAnyDamage
  (params (Damage :type Float%20%28single-precision%29) (DamageType :type Damage%20Type%20Object%20Reference) (InstigatedBy :type Controller%20Object%20Reference) (DamageCauser :type Actor%20Object%20Reference))
  (bind _output_get (Variables|Default|SetCurentHP (- (Variables|Default|GetCurentHP) Damage)))
  (Default|DrillDamaged (Variables|/Game/EnableA/Game/HUDInGame/BPC_AllUMGInGame.BPC_AllUMGInGame_C|GetRefWInGame (Variables|/Game/EnableA/Game/HUDInGame/BP_HUDInGame.BP_HUDInGame_C|GetBPC_AllUMGInGame (Variables|Default|GetRef%20BP%20HUDIn%20Game))) (Variables|Default|GetDrillMaxHP) _output_get)
  (if (<= _output_get 0.0)
    (Development|PrintString "mission failure 
you will die" true true "(R=0.843359,G=0.000000,B=1.000000,A=1.000000)" 2e+01)
    (bind _asbp_pawn_play (Utilities|Casting|CastToBP_PawnPlay (Game|Player|GetPlayerPawn 0)))
    (Utilities|FlowControl|DoOnce false
      (:Completed
        (Game|Damage|ApplyDamage _asbp_pawn_play 4e+01 0 0)
        (Default|YOUWILLDIE _asbp_pawn_play 5e+01)
        (Actor|DestroyActor)))))

(fn ConstructionScript)