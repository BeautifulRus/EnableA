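; BP_Enemy2 is an enemy character that sets its size and stats at spawn.
; BeginPlay switches on a random integer between a smaller, faster variant and a larger, tougher, slower one, though RandomInteger(1) only ever yields the first.
; Overlapping BP_PawnPlay overwrites current HP with that pawn's Damage minus Armor rather than subtracting it, with a note to cast to a projectile instead.
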(event EventBeginPlay
  ;[1 1 1] Придание размера юниту при спавне
  (switch int (Math|Random|RandomInteger 1)
    (:0
      (Transformation|SetActorRelativeScale3D "3.000000,3.000000,3.000000")
      (bind _output_get (Variables|GetDamage|SetMaxHP 1.3e+02))
      (Variables|GetDamage|SetCurentHP _output_get)
      (Variables|GetDamage|SetArmor 0.0)
      (Variables|/Script/Engine.CharacterMovementComponent|SetMaxWalkSpeed (Variables|Character|GetCharacterMovement) 9e+02))
    (:1
      (Transformation|SetActorRelativeScale3D "5.000000,5.000000,5.000000")
      (bind _output_get_2 (Variables|GetDamage|SetMaxHP 3.7e+02))
      (Variables|GetDamage|SetCurentHP _output_get_2)
      (Variables|GetDamage|SetArmor 0.0)
      (Variables|/Script/Engine.CharacterMovementComponent|SetMaxWalkSpeed (Variables|Character|GetCharacterMovement) 6e+02))))

(event Collision|EventActorBeginOverlap
  (params (OtherActor :type Actor%20Object%20Reference))
  (bind _asbp_pawn_play (Utilities|Casting|CastToBP_PawnPlay OtherActor)) ; заменить каст на каст проджектайла
  (Variables|GetDamage|SetCurentHP (- (Variables|/Game/EnableA/Game/Core/HeroCore/BP_PawnPlay.BP_PawnPlay_C|GetDamage _asbp_pawn_play) (Variables|GetDamage|GetArmor))))

(event EventTick
  (params (DeltaSeconds :type Float%20%28single-precision%29)))

(fn ConstructionScript)