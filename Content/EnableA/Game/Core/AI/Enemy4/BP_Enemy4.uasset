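; BP_Enemy4 is a suicide-bomber style enemy character that damages the player at close range.
; On BeginPlay it loops a run animation and caches the player pawn; chase logic is not in this graph.
; When the player enters its sphere, it stops walking, plays an explosion animation and applies full radial damage after a one-second delay.
; Incoming damage reduces its HP and destroys it at zero; the explosion itself does not destroy it.
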(event OnComponentBeginOverlap(Sphere)
  (params (OverlappedComponent :type Primitive%20Component%20Object%20Reference) (OtherActor :type Actor%20Object%20Reference) (OtherComp :type Primitive%20Component%20Object%20Reference) (OtherBodyIndex :type Integer) (bFromSweep :type Boolean) (SweepResult :type Hit%20Result%20Structure%20%28by%20ref%29))
  ;[1 1 1] Наносит урон игроку
  (Utilities|Casting|CastToBP_PawnPlay OtherActor)
  (Variables|/Script/Engine.CharacterMovementComponent|SetMaxWalkSpeed (Variables|Character|GetCharacterMovement) 0.0)
  (Components|Animation|PlayAnimation (Variables|Character|GetMesh) "/Game/EnableA/Game/Core/AI/Enemy4/BugBOMB_meshanimationUV_Anim_explosion_BugBOMB.BugBOMB_meshanimationUV_Anim_explosion_BugBOMB" false)
  (Utilities|FlowControl|Delay 1.0)
  (Game|Damage|ApplyRadialDamage (Variables|SetDamage|GetDamage) (Transformation|GetActorLocation) 2e+02 0 0 0 0 true "ECC_GameTraceChannel1"))

(event EventBeginPlay
  (Components|Animation|PlayAnimation (Variables|Character|GetMesh) "/Game/EnableA/Game/Core/AI/Enemy1/Animations/scorp_run.scorp_run" true)
  (bind _asbp_pawn_play (Utilities|Casting|CastToBP_PawnPlay (Game|Player|GetPlayerPawn 0)))
  (Variables|Default|SetRef%20BP%20Pawn%20Play _asbp_pawn_play))

(event Game|Damage|EventAnyDamage
  (params (Damage :type Float%20%28single-precision%29) (DamageType :type Damage%20Type%20Object%20Reference) (InstigatedBy :type Controller%20Object%20Reference) (DamageCauser :type Actor%20Object%20Reference))
  ;[1 1 1] Получает по хлебалу
  (Variables|GetDamage|SetCurentHP (- (Variables|GetDamage|GetCurentHP) Damage))
  (if (<= (Variables|GetDamage|GetCurentHP) 0.0)
    (Actor|DestroyActor)))

(fn ConstructionScript)