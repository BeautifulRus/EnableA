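; BP_Enemy4 is a scorpion enemy that fights the player pawn in melee.
; BeginPlay randomly picks one of three size tiers, setting HP, armor, speed, damage and cooldown, and adds a red circle sprite.
; Sphere overlaps handle pistol hits, subtracting player damage minus armor from HP and destroying it at zero.
; Player overlap starts a delayed, animated attack loop gated by cooldown, repeating while HeroOnCollision, which any overlap sets, stays true.
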(event OnComponentBeginOverlap(Sphere)
  (params (OverlappedComponent :type Primitive%20Component%20Object%20Reference) (OtherActor :type Actor%20Object%20Reference) (OtherComp :type Primitive%20Component%20Object%20Reference) (OtherBodyIndex :type Integer) (bFromSweep :type Boolean) (SweepResult :type Hit%20Result%20Structure%20%28by%20ref%29))
  (bind _ref_bp_pawn_play (Variables|Default|GetRef%20BP%20Pawn%20Play))
  (bind _armor (Variables|GetDamage|GetArmor))
  (bind _damage (Variables|/Game/EnableA/Game/Core/HeroCore/BP_PawnPlay.BP_PawnPlay_C|GetDamage _ref_bp_pawn_play))
  (bind _returnvalue (- _damage _armor))
  (Variables|Default|SetHeroOnCollision true)
  (Utilities|Casting|CastToBP_PistolProjectileMovement OtherActor
    (:then
      (if (not (<= _returnvalue 0.0))
        (Variables|GetDamage|SetCurentHP (- (Variables|GetDamage|GetCurentHP) _returnvalue))
        (if (<= (Variables|GetDamage|GetCurentHP) 0.0)
          (Actor|DestroyActor))))
    (:CastFailed
      (Utilities|Casting|CastToBP_PawnPlay OtherActor)
      (if (Variables|SetDamage|GetIsAttackReady)
        (Utilities|FlowControl|Sequence :!label _label
          (:then_0
            (Utilities|FlowControl|Delay 1.0) ; время для анимации атаки
            (Default|HeroDamadged/ShieldLogic (Variables|Default|GetRef%20BP%20Pawn%20Play) (Variables|SetDamage|GetDamage))
            (Components|Animation|PlayAnimation (Variables|Character|GetMesh) "/Game/EnableA/Game/Core/AI/AIAnimationsAndMaterials/Enemy1/Animations/scorp_run.scorp_run" true)
            (Variables|SetDamage|SetIsAttackReady false)
            (Utilities|FlowControl|Delay (Variables|SetDamage|GetAttackCooldown))
            (Variables|SetDamage|SetIsAttackReady true)
            (if (Variables|Default|GetHeroOnCollision)
              (goto _label)))
          (:then_1
            (Components|Animation|PlayAnimation (Variables|Character|GetMesh) "/Game/EnableA/Game/Core/AI/AIAnimationsAndMaterials/Enemy1/Animations/scorp_atack_1.scorp_atack_1" false)))))))

(event OnComponentEndOverlap(Sphere)
  (params (OverlappedComponent :type Primitive%20Component%20Object%20Reference) (OtherActor :type Actor%20Object%20Reference) (OtherComp :type Primitive%20Component%20Object%20Reference) (OtherBodyIndex :type Integer))
  (Variables|Default|SetHeroOnCollision false))

(event EventBeginPlay
  (Components|Animation|PlayAnimation (Variables|Character|GetMesh) "/Game/EnableA/Game/Core/AI/AIAnimationsAndMaterials/Enemy1/Animations/scorp_run.scorp_run" true)
  (bind _asbp_pawn_play (Utilities|Casting|CastToBP_PawnPlay (Game|Player|GetPlayerPawn 0)))
  (Variables|Default|SetRef%20BP%20Pawn%20Play _asbp_pawn_play)
  ;[1 1 1] Придание размера юниту при спавне
  (switch int (Math|Random|RandomInteger 3)
    (:0
      (Transformation|SetActorRelativeScale3D "3.000000,3.000000,3.000000")
      (Variables|GetDamage|SetCurentHP 2e+02)
      (Variables|GetDamage|SetArmor 3.0)
      (Variables|/Script/Engine.CharacterMovementComponent|SetMaxWalkSpeed (Variables|Character|GetCharacterMovement) 4e+02)
      (Variables|SetDamage|SetDamage 2e+01)
      (Variables|SetDamage|SetAttackCooldown 0.3)
      (bind _returnvalue (Game|AddComponentbyClass "/Script/Paper2D.PaperSpriteComponent" false))
      (Transformation|AttachComponentToComponent _returnvalue "None" "KeepRelative" "KeepRelative" "KeepRelative" true)
      (Rendering|Components|Sprite|SetSprite _returnvalue "/Game/EnableA/Game/HUDInGame/ChildsInGameWidget/Mimimap/T_RedCircle_Sprite.T_RedCircle_Sprite")
      (Transformation|SetRelativeTransform _returnvalue (Math|Transform|MakeTransform "0.0,0.0,500.0" "0, 0,90.000000" "0.250000,0.250000,0.250000") false true))
    (:1
      (Transformation|SetActorRelativeScale3D "6.000000,6.000000,6.000000")
      (Variables|GetDamage|SetCurentHP 5e+02)
      (Variables|GetDamage|SetArmor 1e+01)
      (Variables|/Script/Engine.CharacterMovementComponent|SetMaxWalkSpeed (Variables|Character|GetCharacterMovement) 3e+02)
      (Variables|SetDamage|SetDamage 5e+01)
      (Variables|SetDamage|SetAttackCooldown 0.5)
      (bind _returnvalue_2 (Game|AddComponentbyClass "/Script/Paper2D.PaperSpriteComponent" false))
      (Transformation|AttachComponentToComponent _returnvalue_2 "None" "KeepRelative" "KeepRelative" "KeepRelative" true)
      (Rendering|Components|Sprite|SetSprite _returnvalue_2 "/Game/EnableA/Game/HUDInGame/ChildsInGameWidget/Mimimap/T_RedCircle_Sprite.T_RedCircle_Sprite")
      (Transformation|SetRelativeTransform _returnvalue_2 (Math|Transform|MakeTransform "0.0,0.0,250.000000" "0, 0,90.000000" "0.180000,0.180000,0.180000") false true))
    (:2
      (Transformation|SetActorRelativeScale3D "12.000000,12.000000,12.000000")
      (Variables|GetDamage|SetCurentHP 8e+02)
      (Variables|GetDamage|SetArmor 25.0)
      (Variables|/Script/Engine.CharacterMovementComponent|SetMaxWalkSpeed (Variables|Character|GetCharacterMovement) 1.5e+02)
      (Variables|SetDamage|SetDamage 65.0)
      (Variables|SetDamage|SetAttackCooldown 1.3)
      (bind _returnvalue_3 (Game|AddComponentbyClass "/Script/Paper2D.PaperSpriteComponent" false))
      (Transformation|AttachComponentToComponent _returnvalue_3 "None" "KeepRelative" "KeepRelative" "KeepRelative" true)
      (Rendering|Components|Sprite|SetSprite _returnvalue_3 "/Game/EnableA/Game/HUDInGame/ChildsInGameWidget/Mimimap/T_RedCircle_Sprite.T_RedCircle_Sprite")
      (Transformation|SetRelativeTransform _returnvalue_3 (Math|Transform|MakeTransform "0.0,0.0,125.000000" "0, 0,90.000000" "0.120000,0.120000,0.120000") false true))))

(event Collision|EventActorBeginOverlap
  (params (OtherActor :type Actor%20Object%20Reference)))

(fn ConstructionScript)