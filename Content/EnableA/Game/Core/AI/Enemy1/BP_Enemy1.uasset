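; BP_Enemy1 is a scorpion enemy that attacks the player pawn at close range and can be killed.
; BeginPlay loops the run animation and caches the player reference.
; Sphere overlap opens and closes a Gate that re-enters itself after each cooldown, repeating a timed attack animation with delayed damage while the player stays inside.
; Incoming damage is reduced by armor, and the actor is destroyed when health runs out.
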(event OnComponentBeginOverlap(Sphere)
  (params (OverlappedComponent :type Primitive%20Component%20Object%20Reference) (OtherActor :type Actor%20Object%20Reference) (OtherComp :type Primitive%20Component%20Object%20Reference) (OtherBodyIndex :type Integer) (bFromSweep :type Boolean) (SweepResult :type Hit%20Result%20Structure%20%28by%20ref%29))
  ;[1 1 1] Даёт по хлебалу
  (Utilities|Casting|CastToBP_PawnPlay OtherActor)
  (Utilities|FlowControl|Sequence
    (:then_0
      (goto _label Open))
    (:then_1
      (Utilities|FlowControl|Gate true :!label _label
        (:Exit
          (if (Variables|SetDamage|GetIsAttackReady)
            (Utilities|FlowControl|Sequence
              (:then_0
                (Utilities|FlowControl|Delay 1.0) ; время для анимации атаки
                (Game|Damage|ApplyDamage (Variables|Default|GetRef%20BP%20Pawn%20Play) (Variables|SetDamage|GetDamage) 0 0)
                (Components|Animation|PlayAnimation (Variables|Character|GetMesh) "/Game/EnableA/Game/Core/AI/Enemy1/Animations/scorp_run.scorp_run" true)
                (Variables|SetDamage|SetIsAttackReady false)
                (Utilities|FlowControl|Delay (Variables|SetDamage|GetAttackCooldown))
                (Variables|SetDamage|SetIsAttackReady true)
                (goto _label))
              (:then_1
                (Components|Animation|PlayAnimation (Variables|Character|GetMesh) "/Game/EnableA/Game/Core/AI/Enemy1/Animations/scorp_atack_1.scorp_atack_1" false)))))))))

(event OnComponentEndOverlap(Sphere)
  (params (OverlappedComponent :type Primitive%20Component%20Object%20Reference) (OtherActor :type Actor%20Object%20Reference) (OtherComp :type Primitive%20Component%20Object%20Reference) (OtherBodyIndex :type Integer))
  ;[1 1 1] Даёт по хлебалу
  (Utilities|Casting|CastToBP_PawnPlay OtherActor)
  (Utilities|FlowControl|Gate true) ; enters at Close
)

(event EventBeginPlay
  (Components|Animation|PlayAnimation (Variables|Character|GetMesh) "/Game/EnableA/Game/Core/AI/Enemy1/Animations/scorp_run.scorp_run" true)
  (bind _asbp_pawn_play (Utilities|Casting|CastToBP_PawnPlay (Game|Player|GetPlayerPawn 0)))
  (Variables|Default|SetRef%20BP%20Pawn%20Play _asbp_pawn_play))

(event Game|Damage|EventAnyDamage
  (params (Damage :type Float%20%28single-precision%29) (DamageType :type Damage%20Type%20Object%20Reference) (InstigatedBy :type Controller%20Object%20Reference) (DamageCauser :type Actor%20Object%20Reference))
  (bind _armor (Variables|GetDamage|GetArmor))
  (bind _returnvalue (- Damage _armor))
  ;[1 1 1] Получает по хлебалу
  (if (not (<= _returnvalue 0.0))
    (bind _output_get (Variables|GetDamage|SetCurentHP (- (Variables|GetDamage|GetCurentHP) _returnvalue)))
    (if (<= _output_get 0.0)
      (Actor|DestroyActor))))

(fn ConstructionScript)