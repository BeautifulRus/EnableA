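; BP_Enemy5 is a clawed bug enemy that hunts the player pawn, the generator and the drill.
; Tick chases a player inside SphereForRetarget, otherwise heading for the drill once the generator is destroyed, or FlipFlopping between generator and drill.
; Sphere overlaps open per-target Gates that loop an attack: stop, animate, apply delayed damage, then cool down.
; AnyDamage reduces HP and destroys the actor at zero.
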(event OnComponentBeginOverlap(Sphere)
  (params (OverlappedComponent :type Primitive%20Component%20Object%20Reference) (OtherActor :type Actor%20Object%20Reference) (OtherComp :type Primitive%20Component%20Object%20Reference) (OtherBodyIndex :type Integer) (bFromSweep :type Boolean) (SweepResult :type Hit%20Result%20Structure%20%28by%20ref%29))
  (if (not (Variables|Default|GetIsDead))
    (Utilities|Casting|CastToBP_PawnPlay OtherActor
      (:then
        (Variables|Default|SetDon'tMovePlease true)
        (Utilities|FlowControl|Sequence
          (:then_0
            (goto _label Open))
          (:then_1
            (Utilities|FlowControl|Gate true :!label _label
              (:Exit
                (if (Variables|SetDamage|GetIsAttackReady)
                  (Variables|SetDamage|SetIsAttackReady false)
                  (Variables|/Script/Engine.CharacterMovementComponent|SetMaxWalkSpeed (Variables|Character|GetCharacterMovement) 0.0)
                  (Components|Animation|PlayAnimation (Variables|Character|GetMesh) "/Game/EnableA/Game/Core/AI/Enemy5/Buglaws_meshanimationUV_Anim_RootAction.Buglaws_meshanimationUV_Anim_RootAction" false)
                  (Utilities|FlowControl|Delay 0.6) ; время для анимации атаки
                  (Game|Damage|ApplyDamage (Variables|Default|GetRef%20BP%20Pawn%20Play) (Variables|SetDamage|GetDamage) 0 0)
                  (Components|Animation|PlayAnimation (Variables|Character|GetMesh) "/Game/EnableA/Game/Core/AI/Enemy5/Buglaws_meshanimationUV_Anim_walk_Claws.Buglaws_meshanimationUV_Anim_walk_Claws" true)
                  (Variables|/Script/Engine.CharacterMovementComponent|SetMaxWalkSpeed (Variables|Character|GetCharacterMovement) (Variables|Default|GetMaxSpeed))
                  (Utilities|FlowControl|Delay (Variables|SetDamage|GetAttackCooldown))
                  (Variables|SetDamage|SetIsAttackReady true)
                  (goto _label)))))))
      (:CastFailed
        (Utilities|Casting|CastToBP_Generator OtherActor
          (:then
            (Variables|Default|SetDon'tMovePlease true)
            (Utilities|FlowControl|Sequence
              (:then_0
                (goto _label_2 Open))
              (:then_1
                (Utilities|FlowControl|Gate true :!label _label_2
                  (:Exit
                    (if (Variables|SetDamage|GetIsAttackReady)
                      (Variables|SetDamage|SetIsAttackReady false)
                      (Variables|/Script/Engine.CharacterMovementComponent|SetMaxWalkSpeed (Variables|Character|GetCharacterMovement) 0.0)
                      (Components|Animation|PlayAnimation (Variables|Character|GetMesh) "/Game/EnableA/Game/Core/AI/Enemy5/Buglaws_meshanimationUV_Anim_RootAction.Buglaws_meshanimationUV_Anim_RootAction" false)
                      (Utilities|FlowControl|Delay 0.6) ; время для анимации атаки
                      (Game|Damage|ApplyDamage (Variables|/Game/EnableA/Game/Core/HeroCore/BP_PawnPlay.BP_PawnPlay_C|GetRefGenerator (Variables|Default|GetRef%20BP%20Pawn%20Play)) (Variables|SetDamage|GetDamage) 0 0)
                      (Components|Animation|PlayAnimation (Variables|Character|GetMesh) "/Game/EnableA/Game/Core/AI/Enemy5/Buglaws_meshanimationUV_Anim_walk_Claws.Buglaws_meshanimationUV_Anim_walk_Claws" true)
                      (Variables|/Script/Engine.CharacterMovementComponent|SetMaxWalkSpeed (Variables|Character|GetCharacterMovement) (Variables|Default|GetMaxSpeed))
                      (Utilities|FlowControl|Delay (Variables|SetDamage|GetAttackCooldown))
                      (Variables|SetDamage|SetIsAttackReady true)
                      (goto _label_2)))))))
          (:CastFailed
            (Utilities|Casting|CastToBP_Drill OtherActor)
            (Variables|Default|SetDon'tMovePlease true)
            (Utilities|FlowControl|Sequence
              (:then_0
                (goto _label_3 Open))
              (:then_1
                (Utilities|FlowControl|Gate true :!label _label_3
                  (:Exit
                    (if (Variables|SetDamage|GetIsAttackReady)
                      (Variables|SetDamage|SetIsAttackReady false)
                      (Variables|/Script/Engine.CharacterMovementComponent|SetMaxWalkSpeed (Variables|Character|GetCharacterMovement) 0.0)
                      (Components|Animation|PlayAnimation (Variables|Character|GetMesh) "/Game/EnableA/Game/Core/AI/Enemy5/Buglaws_meshanimationUV_Anim_RootAction.Buglaws_meshanimationUV_Anim_RootAction" false)
                      (Utilities|FlowControl|Delay 0.6) ; время для анимации атаки
                      (Game|Damage|ApplyDamage (Variables|/Game/EnableA/Game/Core/HeroCore/BP_PawnPlay.BP_PawnPlay_C|GetRefDrill (Variables|Default|GetRef%20BP%20Pawn%20Play)) (Variables|SetDamage|GetDamage) 0 0)
                      (Components|Animation|PlayAnimation (Variables|Character|GetMesh) "/Game/EnableA/Game/Core/AI/Enemy5/Buglaws_meshanimationUV_Anim_walk_Claws.Buglaws_meshanimationUV_Anim_walk_Claws" true)
                      (Variables|/Script/Engine.CharacterMovementComponent|SetMaxWalkSpeed (Variables|Character|GetCharacterMovement) (Variables|Default|GetMaxSpeed))
                      (Utilities|FlowControl|Delay (Variables|SetDamage|GetAttackCooldown))
                      (Variables|SetDamage|SetIsAttackReady true)
                      (goto _label_3))))))))))))

(event OnComponentEndOverlap(Sphere)
  (params (OverlappedComponent :type Primitive%20Component%20Object%20Reference) (OtherActor :type Actor%20Object%20Reference) (OtherComp :type Primitive%20Component%20Object%20Reference) (OtherBodyIndex :type Integer))
  (Utilities|Casting|CastToBP_PawnPlay OtherActor
    (:then
      (Variables|Default|SetDon'tMovePlease false)
      (Utilities|FlowControl|Gate true) ; enters at Close
    )
    (:CastFailed
      (Utilities|Casting|CastToBP_Generator OtherActor
        (:then
          (Variables|Default|SetDon'tMovePlease false)
          (Utilities|FlowControl|Gate true) ; enters at Close
        )
        (:CastFailed
          (Utilities|Casting|CastToBP_Drill OtherActor)
          (Variables|Default|SetDon'tMovePlease false)
          (Utilities|FlowControl|Gate true) ; enters at Close
        )))))

(event EventBeginPlay
  (bind _returnvalue (Pawn|GetController))
  (Variables|Default|SetMaxSpeed (Class|MovementComponent|GetMaxSpeed (Variables|Character|GetCharacterMovement)))
  (Components|Animation|PlayAnimation (Variables|Character|GetMesh) "/Game/EnableA/Game/Core/AI/Enemy5/Buglaws_meshanimationUV_Anim_walk_Claws.Buglaws_meshanimationUV_Anim_walk_Claws" true)
  (bind _asbp_pawn_play (Utilities|Casting|CastToBP_PawnPlay (Game|Player|GetPlayerPawn 0)))
  (Variables|Default|SetRef%20BP%20Pawn%20Play _asbp_pawn_play)
  (bind _output_get (Variables|Default|SetNewVar_0 (Math|Random|RandomInteger 2)))
  (switch int _output_get
    (:0
      (AI|Navigation|SimpleMovetoActor (Pawn|GetController) (Variables|Default|GetRef%20BP%20Pawn%20Play)))
    (:1
      (Utilities|FlowControl|FlipFlop
        (:A
          (AI|Navigation|SimpleMovetoActor _returnvalue (Variables|/Game/EnableA/Game/Core/HeroCore/BP_PawnPlay.BP_PawnPlay_C|GetRefGenerator (Variables|Default|GetRef%20BP%20Pawn%20Play))) ; движение к генератору
        )
        (:B
          (AI|Navigation|SimpleMovetoActor _returnvalue (Variables|/Game/EnableA/Game/Core/HeroCore/BP_PawnPlay.BP_PawnPlay_C|GetRefDrill (Variables|Default|GetRef%20BP%20Pawn%20Play))) ; движение к буру
        ))
      (Variables|Default|SetDon'tMovePlease false))))

(event EventTick
  (params (DeltaSeconds :type Float%20%28single-precision%29))
  (bind _returnvalue (Pawn|GetController))
  (bind _ref_bp_pawn_play (Variables|Default|GetRef%20BP%20Pawn%20Play))
  (Utilities|Casting|CastToBP_PawnPlay (Utilities|Array|Get(acopy) (Collision|GetOverlappingActors (Variables|Default|GetSphereForRetarget) "/Game/EnableA/Game/Core/HeroCore/BP_PawnPlay.BP_PawnPlay_C" :!class /Script/Engine.PrimitiveComponent))
    (:then
      (AI|Navigation|SimpleMovetoActor (Pawn|GetController) (Variables|Default|GetRef%20BP%20Pawn%20Play)))
    (:CastFailed
      (if (not (Variables|Default|GetDon'tMovePlease))
        (if (Variables|/Game/EnableA/Game/Core/HeroCore/BP_PawnPlay.BP_PawnPlay_C|GetIsGeneratorDestroy (Variables|Default|GetRef%20BP%20Pawn%20Play))
          (AI|Navigation|SimpleMovetoActor _returnvalue (Variables|/Game/EnableA/Game/Core/HeroCore/BP_PawnPlay.BP_PawnPlay_C|GetRefDrill _ref_bp_pawn_play) :!label _label) ; движение к буру
          (else
            (Utilities|FlowControl|FlipFlop
              (:A
                (AI|Navigation|SimpleMovetoActor _returnvalue (Variables|/Game/EnableA/Game/Core/HeroCore/BP_PawnPlay.BP_PawnPlay_C|GetRefGenerator _ref_bp_pawn_play)) ; движение к генератору
              )
              (:B
                (goto _label)))))
        (Variables|Default|SetDon'tMovePlease false)))))

(event Game|Damage|EventAnyDamage
  (params (Damage :type Float%20%28single-precision%29) (DamageType :type Damage%20Type%20Object%20Reference) (InstigatedBy :type Controller%20Object%20Reference) (DamageCauser :type Actor%20Object%20Reference))
  ;[1 1 1] В лицо
  (Development|PrintString (Utilities|String|ToString(Float) Damage))
  (bind _output_get (Variables|GetDamage|SetCurentHP (- (Variables|GetDamage|GetCurentHP) Damage)))
  (if (<= _output_get 0.0)
    (Variables|Default|SetIsDead true)
    (Actor|DestroyActor)))

(fn ConstructionScript)