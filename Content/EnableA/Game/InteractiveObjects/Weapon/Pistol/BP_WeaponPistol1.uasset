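; Semi-automatic pistol weapon that fires single debug-drawn line traces with a cooldown, auto-reloading after a delay when Fire finds an empty magazine.
; Each shot randomly picks a spread variant scaled by heat, raises WeaponBurn, spends ammo and sets random recoil on the player pawn.
; Tick cools and clamps heat, with only a debug print for overheating.
; Trace hits are unused, so no damage is applied here.
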(event EventBeginPlay
  ;[1 1 1 1 95] Это оружие стреляет одиночками с небольшим кд,
  (bind _asbp_hudin_game (Utilities|Casting|CastToBP_HUDInGame (HUD|GetHUD (Game|GetPlayerController 0)))
    (:then
      (|CallParentFunction))
    (:CastFailed
      (Development|PrintString "cast fail 
BP_WeaponPistol1"))))

(event Collision|EventActorBeginOverlap
  (params (OtherActor :type Actor%20Object%20Reference))
  ;[1 1 1 1 95] Это оружие стреляет одиночками с небольшим кд,
  (|CallParentFunction OtherActor) ; This node is disabled and will not be called.\nDrag off pins to build functionality.
)

(event EventTick
  (params (DeltaSeconds :type Float%20%28single-precision%29))
  ;[1 1 1 1 95] Это оружие стреляет одиночками с небольшим кд,
  (Utilities|FlowControl|Sequence
    (:then_0)
    (:then_1
      (|Охлаждениеоружия)
      (|Ограничениевыходанагревавминус
        (:%20then
          (if (|Проверканаперегреворужия)
            (Development|PrintString "перегрев включай эффект ожога на весь экран, пока перегрев не спадёт" true true "(R=1.000000,G=0.047766,B=0.000000,A=1.000000)" 0.0)))))))

(event EventFire
  (params (HeroDamage :type Float%20%28single-precision%29))
  (bind _returnvalue (Transformation|GetActorForwardVector))
  (bind _returnvalue_2 (Transformation|GetActorForwardVector))
  (bind _returnvalue_3 (Transformation|GetActorForwardVector))
  (bind _arrow (Variables|Components|GetArrow))
  (bind _arrow_2 (Variables|Components|GetArrow))
  (bind _arrow_3 (Variables|Components|GetArrow))
  (bind _returnvalue_4 (Transformation|GetWorldLocation _arrow))
  (bind _returnvalue_5 (Transformation|GetWorldLocation _arrow_2))
  (bind _returnvalue_6 (Transformation|GetWorldLocation _arrow_3))
  ;[1 1 1 1 95] Это оружие стреляет одиночками с небольшим кд,
  ;;[1 1 1] Semi
  (if (Variables|Default|GetReadyToShoot)
    (Variables|Default|SetReadyToShoot false)
    (if (== (Variables|Default|GetNumberOf%20Remaining%20AmmoInTheMagazine) 0)
      (Utilities|FlowControl|Delay (Variables|Default|GetRemovalAndReloading))
      (Variables|Default|SetNumberOf%20Remaining%20AmmoInTheMagazine (Variables|Default|GetMagazineCapacity))
      (Variables|Default|SetReadyToShoot true)
      (else
        (switch int (Math|Random|RandomInteger 2)
          (:0
            ;;[1 1 1] Логика разбро
            ;;;[1 1 1] Вариант 1
            (Variables|Default|SetTimesDerivation (- (/ (Variables|Default|GetWeaponBurn) 3e+02) (Variables|Default|GetDerivation%20)))
            (Collision|LineTraceByChannel _returnvalue_5 (+ (* (Math|Vector|MakeVector (+ (.x _returnvalue) (Math|Random|RandomFloatinRange (* (Variables|Default|GetTimesDerivation) -1.0) (Variables|Default|GetTimesDerivation))) (+ (.y _returnvalue) (Math|Random|RandomFloatinRange (* (Variables|Default|GetTimesDerivation) -1.0) (Variables|Default|GetTimesDerivation))) (.z _returnvalue)) 1.3e+03) _returnvalue_5) "TraceTypeQuery1" false 0 "Persistent"))
          (:1
            ;;;[1 1 1] Вариант2
            (Variables|Default|SetTimesDerivation (+ (Variables|Default|GetDerivation%20) (/ (Variables|Default|GetWeaponBurn) 3e+02)))
            (Collision|LineTraceByChannel _returnvalue_4 (+ (* (Math|Vector|MakeVector (+ (.x _returnvalue_2) (Math|Random|RandomFloatinRange (* (Variables|Default|GetTimesDerivation) -1.0) (Variables|Default|GetTimesDerivation))) (+ (.y _returnvalue_2) (Math|Random|RandomFloatinRange (* (Variables|Default|GetTimesDerivation) -1.0) (Variables|Default|GetTimesDerivation))) (.z _returnvalue_2)) 1.3e+03) _returnvalue_4) "TraceTypeQuery1" false 0 "Persistent"))
          (:2
            ;;;[1 1 1] Вариант3
            (Variables|Default|SetTimesDerivation (+ (Variables|Default|GetDerivation%20) (/ (Variables|Default|GetWeaponBurn) 3e+02)))
            (Collision|LineTraceByChannel _returnvalue_6 (+ (* (Math|Vector|MakeVector (- (.x _returnvalue_3) (Math|Random|RandomFloatinRange (* (Variables|Default|GetTimesDerivation) -1.0) (Variables|Default|GetTimesDerivation))) (+ (.y _returnvalue_3) (Math|Random|RandomFloatinRange (* (Variables|Default|GetTimesDerivation) -1.0) (Variables|Default|GetTimesDerivation))) (.z _returnvalue_3)) 1.3e+03) _returnvalue_6) "TraceTypeQuery1" false 0 "Persistent")))
        (|Повышениенагреваоружия)
        (Math|Integer|DecrementInt (Variables|Default|GetNumberOf%20Remaining%20AmmoInTheMagazine)
          (:%20%20
            (Utilities|FlowControl|Delay (Variables|Default|GetSpeedShooting))
            (Variables|Default|SetReadyToShoot true)
            (Variables|/Game/EnableA/Game/Core/BP_PawnPlay.BP_PawnPlay_C|SetWeaponRecoil (Variables|Default|GetRefBPPawnPlay) (Math|Vector|MakeVector (Math|Random|RandomFloatinRange (* (.x (Variables|Default|GetWeaponRecoil)) -1.0) (.x (Variables|Default|GetWeaponRecoil))) (Math|Random|RandomFloatinRange (* (.y (Variables|Default|GetWeaponRecoil)) -1.0) (.y (Variables|Default|GetWeaponRecoil))) 0.0))))))))

(fn ConstructionScript
  (|CallParentFunction))