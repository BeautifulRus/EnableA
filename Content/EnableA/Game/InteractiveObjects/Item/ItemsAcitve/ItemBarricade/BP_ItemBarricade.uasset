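; BP_ItemBarricade is an active item that places a barricade in front of the player pawn.
; Its qwer event spawns BP_MeshFromBarricade ahead of the pawn's Arrow component, using the arrow's rotation, a fixed height and an enlarged scale.
; The IsItemReady flag and a Delay of ItemCoolDown gate reuse, and a debug message prints when the item is not ready.
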(event Custom|qwer
  (bind _refbp_pawn_play (Variables|Default|GetRefBP%20Pawn%20Play))
  (bind _returnvalue (Transformation|GetActorForwardVector _refbp_pawn_play))
  (bind _arrow (Variables|/Game/EnableA/Game/Core/BP_PawnPlay.BP_PawnPlay_C|GetArrow _refbp_pawn_play))
  (bind _returnvalue_2 (Transformation|GetWorldLocation _arrow))
  (bind _returnvalue_3 (* _returnvalue 5e+02))
  (bind _returnvalue_4 (+ _returnvalue_2 _returnvalue_3))
  (if (Variables|Default|GetIsItemReady)
    (Game|SpawnActorfromClass "/Game/EnableA/Game/InteractiveObjects/Item/ItemsAcitve/ItemBarricade/BP_MeshFromBarricade.BP_MeshFromBarricade_C" (Math|Transform|MakeTransform (Math|Vector|MakeVector (.x _returnvalue_4) (.y _returnvalue_4) 1e+02) (Transformation|GetWorldRotation _arrow) "2.000000,2.000000,2.000000") "AdjustIfPossibleButAlwaysSpawn" 0 0)
    (Variables|Default|SetIsItemReady false)
    (Utilities|FlowControl|Delay (Variables|Default|GetItemCoolDown))
    (Variables|Default|SetIsItemReady true)
    (else
      (Development|PrintString "item is not ready"))))

(event EventBeginPlay)

(event Collision|EventActorBeginOverlap
  (params (OtherActor :type Actor%20Object%20Reference)))

(event EventTick
  (params (DeltaSeconds :type Float%20%28single-precision%29)))

(fn ConstructionScript
  (|CallParentFunction))