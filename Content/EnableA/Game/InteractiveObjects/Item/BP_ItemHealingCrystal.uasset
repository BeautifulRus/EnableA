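; Healing crystal item that passively regenerates health on the referenced player pawn and can be upgraded through grades.
; Tick adds HealthRegeneration to the pawn's current health while it is below a hardcoded 900, per frame without delta-time scaling.
; UpgradeItem increments GradeSystem and switches on it to set one of five rising regeneration amounts, printing a Russian max-level message for any grade outside that range.
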(event Custom|UpgradeItem
  ;[1 1 1] GradeSystem
  (bind _result (Math|Integer|IncrementInt (Variables|Default|GetGradeSystem))
    (:%20%20
      (switch int _result
        (:Default
          (Development|PrintString "Это максимум этого предмета"))
        (:0
          (Variables|Default|Set++HealthRegeneration 1.0))
        (:1
          (Variables|Default|Set++HealthRegeneration 2.5))
        (:2
          (Variables|Default|Set++HealthRegeneration 3.5))
        (:3
          (Variables|Default|Set++HealthRegeneration 4.3))
        (:4
          (Variables|Default|Set++HealthRegeneration 5.0))))))

(event EventBeginPlay)

(event Collision|EventActorBeginOverlap
  (params (OtherActor :type Actor%20Object%20Reference)))

(event EventTick
  (params (DeltaSeconds :type Float%20%28single-precision%29))
  (bind _refbp_pawn_play (Variables|Default|GetRefBP%20Pawn%20Play))
  (if (not (>= (Variables|/Game/EnableA/Game/Core/HeroCore/BP_PawnPlay.BP_PawnPlay_C|GetHealthCurent _refbp_pawn_play) 9e+02))
    (Variables|/Game/EnableA/Game/Core/HeroCore/BP_PawnPlay.BP_PawnPlay_C|SetHealthCurent _refbp_pawn_play (+ (Variables|Default|Get++HealthRegeneration) (Variables|/Game/EnableA/Game/Core/HeroCore/BP_PawnPlay.BP_PawnPlay_C|GetHealthCurent _refbp_pawn_play)))))

(fn ConstructionScript
  (|CallParentFunction))