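; Steam pack active item that trades hero health for a temporary boost to movement speed, health regeneration, dash cooldown and damage.
; ItemUse adds Armor to the HP cost passed as damage, saves and modifies the pawn's stats, then restores the saved values after the active time.
; A ready flag blocks reuse until the subsequent cooldown ends.
; UpgradeItem increments the grade to select preset costs, modifiers and timings.
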(event Custom|ItemUse
  (bind _refbp_pawn_play (Variables|Default|GetRefBP%20Pawn%20Play))
  (bind _refbp_pawn_play_2 (Variables|Default|GetRefBP%20Pawn%20Play))
  (bind _refbp_pawn_play_3 (Variables|Default|GetRefBP%20Pawn%20Play))
  (bind _refbp_pawn_play_4 (Variables|Default|GetRefBP%20Pawn%20Play))
  (bind _refbp_pawn_play_5 (Variables|Default|GetRefBP%20Pawn%20Play))
  (bind _refbp_pawn_play_6 (Variables|Default|GetRefBP%20Pawn%20Play))
  (if (Variables|Default|GetIsItemReady)
    (Utilities|FlowControl|Sequence
      (:then_0
        ;[1 1 1] 100 урона в хп героя
        (Default|HeroDamaged/HealthLogic _refbp_pawn_play_5 (+ (Variables|Default|Get--HP) (Variables|/Game/EnableA/Game/Core/HeroCore/BP_PawnPlay.BP_PawnPlay_C|GetArmor _refbp_pawn_play_5))))
      (:then_1
        ;[1 1 1] Повышение скорости персонажа
        (Variables|Default|SetHeroMovementSpeedBefore (Variables|/Game/EnableA/Game/Core/HeroCore/BP_PawnPlay.BP_PawnPlay_C|GetHeroMovementSpeed _refbp_pawn_play_6))
        (Variables|/Game/EnableA/Game/Core/HeroCore/BP_PawnPlay.BP_PawnPlay_C|SetHeroMovementSpeed _refbp_pawn_play_6 (* (Variables|/Game/EnableA/Game/Core/HeroCore/BP_PawnPlay.BP_PawnPlay_C|GetHeroMovementSpeed _refbp_pawn_play_6) (Variables|Default|Get++MovementSpeed)))
        (Default|SteamPuckUse _refbp_pawn_play_6))
      (:then_2
        ;[1 1 1] Регенерация хп
        (Variables|Default|SetHealthRegenerationBefore (Variables|/Game/EnableA/Game/Core/HeroCore/BP_PawnPlay.BP_PawnPlay_C|GetHealthRegeneration _refbp_pawn_play_2))
        (Variables|/Game/EnableA/Game/Core/HeroCore/BP_PawnPlay.BP_PawnPlay_C|SetHealthRegeneration _refbp_pawn_play_2 (+ (Variables|/Game/EnableA/Game/Core/HeroCore/BP_PawnPlay.BP_PawnPlay_C|GetHealthRegeneration _refbp_pawn_play_2) (Variables|Default|Get++HealthRegeneration))))
      (:then_3
        ;[1 1 1] Скорость перезарядки рывка
        (Variables|Default|SetDashCooldownBefore (Variables|/Game/EnableA/Game/Core/HeroCore/BP_PawnPlay.BP_PawnPlay_C|GetDashCooldown _refbp_pawn_play_3))
        (Variables|/Game/EnableA/Game/Core/HeroCore/BP_PawnPlay.BP_PawnPlay_C|SetDashCooldown _refbp_pawn_play_3 (* (Variables|/Game/EnableA/Game/Core/HeroCore/BP_PawnPlay.BP_PawnPlay_C|GetDashCooldown _refbp_pawn_play_3) (Variables|Default|Get++DashCooldown))))
      (:then_4
        ;[1 1 1] Увеличение урона
        (Variables|Default|SetDamageBefore (Variables|/Game/EnableA/Game/Core/HeroCore/BP_PawnPlay.BP_PawnPlay_C|GetDamage _refbp_pawn_play))
        (Variables|/Game/EnableA/Game/Core/HeroCore/BP_PawnPlay.BP_PawnPlay_C|SetDamage _refbp_pawn_play (* (Variables|/Game/EnableA/Game/Core/HeroCore/BP_PawnPlay.BP_PawnPlay_C|GetDamage _refbp_pawn_play) (Variables|Default|Get++Damage))))
      (:then_5
        (Variables|Default|SetIsItemReady false) ; запрет на повторное использование \nпредмета, ибо иначе его \nможно прожимать каждые 14 секунд\nпосле активации
        (Utilities|FlowControl|Delay (Variables|Default|GetActiveTimeItem)) ; активное время предмета
        ;[1 1 1] Возвращение параметрам обычных значений
        (Utilities|FlowControl|Sequence
          (:then_0
            (Variables|/Game/EnableA/Game/Core/HeroCore/BP_PawnPlay.BP_PawnPlay_C|SetHeroMovementSpeed _refbp_pawn_play_4 (Variables|Default|GetHeroMovementSpeedBefore))
            (Default|SteamPuckUse _refbp_pawn_play_4))
          (:then_1
            (Variables|/Game/EnableA/Game/Core/HeroCore/BP_PawnPlay.BP_PawnPlay_C|SetHealthRegeneration _refbp_pawn_play_4 (Variables|Default|GetHealthRegenerationBefore)))
          (:then_2
            (Variables|/Game/EnableA/Game/Core/HeroCore/BP_PawnPlay.BP_PawnPlay_C|SetDashCooldown _refbp_pawn_play_4 (Variables|Default|GetDashCooldownBefore)))
          (:then_3
            (Variables|/Game/EnableA/Game/Core/HeroCore/BP_PawnPlay.BP_PawnPlay_C|SetDamage _refbp_pawn_play_4 (Variables|Default|GetDamageBefore)))
          (:then_4
            ;[1 1 1] Перезарядка предмета
            (Utilities|FlowControl|Delay (Variables|Default|GetItemCoolDown)) ; время перезарядки предмета
            (Variables|Default|SetIsItemReady true)))))))

(event Custom|UpgradeItem
  ;[1 1 1] GradeSystem
  (bind _result (Math|Integer|IncrementInt (Variables|Default|GetGradeSystem))
    (:%20%20
      (switch int _result
        (:Default
          (Development|PrintString "Это максимум этого предмета"))
        (:0
          (Variables|Default|Set--HP 1e+02)
          (Variables|Default|Set++MovementSpeed 1.15)
          (Variables|Default|Set++HealthRegeneration 1.0)
          (Variables|Default|Set++DashCooldown 0.8)
          (Variables|Default|Set++Damage 1.2)
          (Variables|Default|SetActiveTimeItem 15.0)
          (Variables|Default|SetItemCoolDown 6e+01))
        (:1
          (Variables|Default|Set--HP 85.0)
          (Variables|Default|Set++MovementSpeed 1.18)
          (Variables|Default|Set++HealthRegeneration 2.5)
          (Variables|Default|Set++DashCooldown 0.78)
          (Variables|Default|Set++Damage 1.23)
          (Variables|Default|SetActiveTimeItem 17.0)
          (Variables|Default|SetItemCoolDown 57.0))
        (:2
          (Variables|Default|Set--HP 6e+01)
          (Variables|Default|Set++MovementSpeed 1.21)
          (Variables|Default|Set++HealthRegeneration 5.0)
          (Variables|Default|Set++DashCooldown 0.73)
          (Variables|Default|Set++Damage 1.26)
          (Variables|Default|SetActiveTimeItem 2e+01)
          (Variables|Default|SetItemCoolDown 53.0))
        (:3
          (Variables|Default|Set--HP 1.1e+02)
          (Variables|Default|Set++MovementSpeed 1.45)
          (Variables|Default|Set++HealthRegeneration 4.0)
          (Variables|Default|Set++DashCooldown 0.61)
          (Variables|Default|Set++Damage 1.34)
          (Variables|Default|SetActiveTimeItem 12.0)
          (Variables|Default|SetItemCoolDown 5e+01))
        (:4
          (Variables|Default|Set--HP 1.5e+02)
          (Variables|Default|Set++MovementSpeed 1.55)
          (Variables|Default|Set++HealthRegeneration 4.5)
          (Variables|Default|Set++DashCooldown 0.58)
          (Variables|Default|Set++Damage 1.42)
          (Variables|Default|SetActiveTimeItem 1e+01)
          (Variables|Default|SetItemCoolDown 4e+01))))))

(event EventBeginPlay)

(event Collision|EventActorBeginOverlap
  (params (OtherActor :type Actor%20Object%20Reference)))

(fn ConstructionScript
  (|CallParentFunction))