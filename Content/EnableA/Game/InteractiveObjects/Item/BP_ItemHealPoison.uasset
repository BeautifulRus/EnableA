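; BP_ItemHealPoison is a usable healing item that temporarily boosts the player pawn's health regeneration.
; ItemUse, gated by a ready flag, saves the current regeneration rate, adds the item's bonus, then restores the saved value after the active time.
; A further cooldown delay then re-enables the item.
; UpgradeItem increments the grade counter and switches on it to set the bonus and cooldown.
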(event Custom|ItemUse
  (bind _refbp_pawn_play (Variables|Default|GetRefBP%20Pawn%20Play))
  (if (Variables|Default|GetIsItemReady)
    (Variables|Default|SetHealthRegenerationBefore (Variables|/Game/EnableA/Game/Core/BP_PawnPlay.BP_PawnPlay_C|GetHealthRegeneration _refbp_pawn_play))
    (Variables|/Game/EnableA/Game/Core/BP_PawnPlay.BP_PawnPlay_C|SetHealthRegeneration _refbp_pawn_play (+ (Variables|/Game/EnableA/Game/Core/BP_PawnPlay.BP_PawnPlay_C|GetHealthRegeneration _refbp_pawn_play) (Variables|Default|Get++HealthRegeneration)))
    (Variables|Default|SetIsItemReady false)
    (Utilities|FlowControl|Delay (Variables|Default|GetActiveTimeItem))
    (Variables|/Game/EnableA/Game/Core/BP_PawnPlay.BP_PawnPlay_C|SetHealthRegeneration (Variables|Default|GetRefBP%20Pawn%20Play) (Variables|Default|GetHealthRegenerationBefore))
    (Utilities|FlowControl|Delay (Variables|Default|GetItemCoolDown))
    (Variables|Default|SetIsItemReady true)))

(event Custom|UpgradeItem
  ;[1 1 1] GradeSystem
  (bind _result (Math|Integer|IncrementInt (Variables|Default|GetGradeSystem))
    (:%20%20
      (switch int _result
        (:0
          (Variables|Default|Set++HealthRegeneration 1e+01)
          (Variables|Default|SetItemCoolDown 8e+01))
        (:1
          (Variables|Default|Set++HealthRegeneration 13.0)
          (Variables|Default|SetItemCoolDown 9e+01))
        (:2
          (Variables|Default|Set++HealthRegeneration 17.0)
          (Variables|Default|SetItemCoolDown 1e+02))
        (:3
          (Variables|Default|Set++HealthRegeneration 4.0)
          (Variables|Default|SetItemCoolDown 6e+01))
        (:4
          (Variables|Default|Set++HealthRegeneration 4.5)
          (Variables|Default|SetItemCoolDown 55.0))))))

(event EventBeginPlay)

(event Collision|EventActorBeginOverlap
  (params (OtherActor :type Actor%20Object%20Reference)))

(event EventTick
  (params (DeltaSeconds :type Float%20%28single-precision%29)))

(fn ConstructionScript
  (|CallParentFunction))