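; BP_ItemGranade is a usable, upgradeable grenade item for the player pawn.
; On use, if the item is ready, it spawns BP_MeshForItemGranade at the pawn's Arrow transform.
; Upgrades increment GradeSystem and switch to set cooldown and hero-damage splash multiplier, printing a Russian max-level message outside the handled grades.
; The cooldown reset sequence and splash damage calculation are present but disconnected.
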(event Custom|ItemUse
  (if (Variables|Default|GetIsItemReady)
    (Game|SpawnActorfromClass "/Game/EnableA/Game/InteractiveObjects/Item/ItemGranade/BP_MeshForItemGranade.BP_MeshForItemGranade_C" (Transformation|GetWorldTransform (Variables|/Game/EnableA/Game/Core/HeroCore/BP_PawnPlay.BP_PawnPlay_C|GetArrow (Variables|Default|GetRefBP%20Pawn%20Play))) "Undefined" 0 0)))

(event Custom|UpgradeItem
  ;[1 1 1] GradeSystem
  (bind _result (Math|Integer|IncrementInt (Variables|Default|GetGradeSystem))
    (:%20%20
      (switch int _result
        (:Default
          (Development|PrintString "Это максимум этого предмета"))
        (:0
          (Variables|Default|SetItemCoolDown 6e+01)
          (Variables|Default|SetSplashDamageFromHeroDamagePercent 3.5))
        (:1
          (Variables|Default|SetItemCoolDown 57.0)
          (Variables|Default|SetSplashDamageFromHeroDamagePercent 4.5))
        (:2
          (Variables|Default|SetItemCoolDown 53.0)
          (Variables|Default|SetSplashDamageFromHeroDamagePercent 5.8))
        (:3
          (Variables|Default|SetItemCoolDown 5e+01)
          (Variables|Default|SetSplashDamageFromHeroDamagePercent 6.4))
        (:4
          (Variables|Default|SetItemCoolDown 4e+01)
          (Variables|Default|SetSplashDamageFromHeroDamagePercent 7.0))))))

(event EventBeginPlay)

(event Collision|EventActorBeginOverlap
  (params (OtherActor :type Actor%20Object%20Reference)))

(event EventTick
  (params (DeltaSeconds :type Float%20%28single-precision%29)))

(fn ConstructionScript
  (|CallParentFunction))